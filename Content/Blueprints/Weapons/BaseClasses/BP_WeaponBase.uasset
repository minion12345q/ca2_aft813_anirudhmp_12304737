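; Base weapon Blueprint providing shared ammo, cooldown, hitscan and cosmetic logic, with empty fire and reload events.
; Helpers auto-reload empty magazines, time fire readiness and line trace damage into CBP_Health components.
; Equip and Unequip play animations, then both poll IsUnequipComplete through Delay loops before toggling mesh visibility and collision.
; Cosmetic events eject physics casings at randomized speed and animate the charging handle by timeline.
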(event Custom|Animate%20Charger
  ;[1 1 1] This custom event will be called to animate the charger. It will affect no other functionality
  (bind _charging_handle_ (Timeline|Timeline PlayFromStart)
    (:Update
      (Transformation|SetRelativeLocation (Variables|Default|GetSM_Charger) (Math|Vector|Lerp(Vector) "-0.270000,0.000000,-0.230000" (Variables|WeaponVisuals|GetChargerMax) _charging_handle_) false false))))

(event Custom|Eject%20Casing
  ;[1 1 1] Spawn Cartridge at spawn location
  (bind _returnvalue (Game|SpawnActorfromClass (Variables|WeaponVisuals|GetCartridge%20Spawn%20Class) (Transformation|GetWorldTransform (Variables|Default|GetCartridgeEjectLoc)) "Undefined" "MultiplyWithRoot" 0 0))
  ;[1 1 1] Add Force to throw cartridge away from the gun
  (bind _asbp_ejected_cartridge_base (Utilities|Casting|CastToBP_EjectedCartridgeBase _returnvalue)
    (:then
      (Default|AddEjectionForceandRotationalRandomness _asbp_ejected_cartridge_base (* (Math|Vector|GetForwardVector (Variables|Default|GetCartridgeEjectLoc)) (CallFunction|GetRandomCartridgeEjectionSpeed)) (CallFunction|GetRandomCartridgeEjectionSpeed)))
    (:CastFailed
      (Development|PrintString "Spawned Cartiridge could not be casted to ejected cartridge base"))))

(event Custom|Reload)

(event Custom|Unequip
  (Components|Animation|PlayAnimation (Variables|Default|GetSkeletalMesh) "/Game/3DAssets/Guns/Barret_Rigged/Barret_Anim_Rig_Barret_Unequip.Barret_Anim_Rig_Barret_Unequip" false)
  (Variables|AnimationTiming|SetisUnequipComplete false)
  (Utilities|FlowControl|Delay 0.05 :!label _label)
  (if (Variables|AnimationTiming|GetisUnequipComplete)
    (CallFunction|UnequippedFunctionality)
    (else
      (goto _label))))

(event Custom|On%20Fire%20Held
  (params (Forward%20Vector :type Vector)))

(event Custom|On%20Fire%20Left)

(event Custom|Start%20Weapon%20Cooldown
  (bind _returnvalue (Utilities|Time|SetTimerbyEvent (delegate Custom|Weapon%20Cooldown) (Variables|WeaponBehavior-Mechanics|GetFiringCoolDown))))

(event Custom|Weapon%20Cooldown
  (Variables|WeaponBehavior-Mechanics|SetIsReadyToFire true)
  (Development|PrintString (Utilities|String|Append "Weapon Cooldown of " (Utilities|String|ToString(Float) (Variables|WeaponBehavior-Mechanics|GetFiringCoolDown)) " seconds is now complete. Weapon Ready to fire") true true "(R=0.765522,G=0.667371,B=1.000000,A=1.000000)" 0.5)
  (Utilities|Time|ClearandInvalidateTimerbyHandle (stale Custom|Start%20Weapon%20Cooldown _returnvalue)))

(event Custom|On%20Fire%20Pressed
  (params (Forward%20Vector :type Vector)))

(event Custom|Equip
  (Components|Animation|PlayAnimation (Variables|Default|GetSkeletalMesh) "/Game/3DAssets/Guns/Barret_Rigged/Barret_Anim_Rig_Barret_Equip.Barret_Anim_Rig_Barret_Equip" false)
  (Variables|AnimationTiming|SetisEquipComplete false)
  (Utilities|FlowControl|Delay 0.05 :!label _label)
  (if (Variables|AnimationTiming|GetisUnequipComplete)
    (CallFunction|EquippedFunctionality)
    (else
      (goto _label))))

(event EventBeginPlay
  (Variables|WeaponBehavior-Ammo|SetCurrent%20Magazine%20Capacity (Variables|WeaponBehavior-Ammo|GetMaximum%20Magazine%20Capacity))
  (Variables|WeaponBehavior-Mechanics|SetIsReadyToFire true)
  (Class|IBPAnimations|EstablishGunReference(Message) (Components|SkeletalMesh|GetAnimInstance (Variables|Default|GetSkeletalMesh)) self))

(event EventUnequipComplete
  ;[1 1 1] Animation Complete Checks
  (Variables|AnimationTiming|SetisUnequipComplete true))

(event EventReloadComplete
  ;[1 1 1] Animation Complete Checks
  (Variables|AnimationTiming|SetisReloadComplete true))

(event EventEquipComplete
  ;[1 1 1] Animation Complete Checks
  (Variables|AnimationTiming|SetisEquipComplete true))

(fn ConstructionScript)

(fn CheckAmmoBeforeFiring
  (if (> (Variables|WeaponBehavior-Ammo|GetCurrent%20Magazine%20Capacity) 0) ; Check to see if magazine is not emplty
    _
    (else
      (bind _is_reload_succesful (CallFunction|ReloadFunctionality))
      (if _is_reload_succesful
        _
        (else
          (return false)))))
  (return true))

(fn ReloadFunctionality
  (if (> (Variables|WeaponBehavior-Ammo|GetTotal%20Ammo) 0)
    (if (> (Variables|WeaponBehavior-Ammo|GetTotal%20Ammo) (Variables|WeaponBehavior-Ammo|GetMaximum%20Magazine%20Capacity))
      (Variables|WeaponBehavior-Ammo|SetTotal%20Ammo (- (Variables|WeaponBehavior-Ammo|GetTotal%20Ammo) (Variables|WeaponBehavior-Ammo|GetMaximum%20Magazine%20Capacity)))
      (Variables|WeaponBehavior-Ammo|SetCurrent%20Magazine%20Capacity (Variables|WeaponBehavior-Ammo|GetMaximum%20Magazine%20Capacity))
      (Development|PrintString (Utilities|String|Append "Reload Complete. " "Total Ammo after reload = " (Utilities|String|ToString(Integer) (Variables|WeaponBehavior-Ammo|GetTotal%20Ammo)) " ||| Current Ammo in Mag After Reload = " (Utilities|String|ToString(Integer) (Variables|WeaponBehavior-Ammo|GetCurrent%20Magazine%20Capacity))))
      (Variables|WeaponBehavior-Mechanics|SetIsReadyToFire true)
      (else
        (Variables|WeaponBehavior-Ammo|SetCurrent%20Magazine%20Capacity (Variables|WeaponBehavior-Ammo|GetTotal%20Ammo))
        (Variables|WeaponBehavior-Ammo|SetTotal%20Ammo 0)
        (Development|PrintString (Utilities|String|Append "Reload Complete. " "Total Ammo after reload = " (Utilities|String|ToString(Integer) (Variables|WeaponBehavior-Ammo|GetTotal%20Ammo)) " ||| Current Ammo in Mag After Reload = " (Utilities|String|ToString(Integer) (Variables|WeaponBehavior-Ammo|GetCurrent%20Magazine%20Capacity))))
        (Variables|WeaponBehavior-Mechanics|SetIsReadyToFire true)))
    (return true)
    (else
      (Development|PrintString "No Total Ammo")
      (return false))))

(fn UnequippedFunctionality
  (bind _skeletalmesh (Variables|Default|GetSkeletalMesh))
  (Rendering|SetVisibility _skeletalmesh false true)
  (Collision|SetCollisionEnabled _skeletalmesh "NoCollision"))

(fn EquippedFunctionality
  (bind _skeletalmesh (Variables|Default|GetSkeletalMesh))
  (Rendering|SetVisibility _skeletalmesh true true)
  (Collision|SetCollisionEnabled _skeletalmesh "QueryAndPhysics"))

(fn GetFiringLocationInfo
  (bind _firingloc (Variables|Default|GetFiringLoc))
  (return (Transformation|GetWorldLocation _firingloc) (Math|Vector|GetForwardVector _firingloc)))

(fn FireRayCast
  (params (Forward%20Vector :type Vector))
  (bind _firingloc (Variables|Default|GetFiringLoc))
  (bind _returnvalue (Transformation|GetWorldLocation _firingloc))
  (bind (_outhit _returnvalue_2) (Collision|LineTraceByChannel _returnvalue (+ _returnvalue (* Forward%20Vector (Variables|WeaponBehavior-Mechanics|GetWeapon%20Range))) "TraceTypeQuery1" false 0 "ForDuration" true "(R=1.000000,G=0.000000,B=0.000000,A=1.000000)" "(R=0.000000,G=1.000000,B=0.000000,A=1.000000)" 2.0))
  (if _returnvalue_2 ; Checking if anything was hit at all
    (Utilities|IsValid (Actor|GetComponentbyClass (.hitactor _outhit) "/Game/Core/Component/CBP_Health.CBP_Health_C") ; Does the hit object contain a valid health component
      (:Is%20Valid
        (Default|TakeDamage (Actor|GetComponentbyClass (.hitactor _outhit) "/Game/Core/Component/CBP_Health.CBP_Health_C") (Variables|WeaponBehavior-Mechanics|GetDamage))
        (Development|PrintString (Utilities|String|Append "Bullet Has Hit Target Actor By Name: " (Utilities|GetDisplayName (.hitactor _outhit)) ". Bullet Has caused " (Utilities|String|ToString(Float) (Variables|WeaponBehavior-Mechanics|GetDamage)) "damage.") true true "(R=0.814583,G=0.377565,B=0.000000,A=1.000000)" 0.5))
      (:Is%20Not%20Valid
        (Development|PrintString (Utilities|String|Append "Bullet Has Hit Target Actor By Name: " (Utilities|GetDisplayName (.hitactor _outhit))) true true "(R=0.666547,G=0.814583,B=0.110376,A=1.000000)" 0.5)))
    (else
      (Development|PrintString "Bullet Did not Hit Anything" true true "(R=0.797917,G=0.644183,B=0.000000,A=1.000000)" 0.2))))

(fn ReduceAmmoAfterFiring
  (Math|Integer|DecrementInt (Variables|WeaponBehavior-Ammo|GetCurrent%20Magazine%20Capacity)))

(fn GetRandomCartridgeEjectionSpeed
  (bind _cartridge_ejection_speed (Variables|WeaponVisuals|GetCartridge%20Ejection%20Speed))
  (bind _returnvalue (* _cartridge_ejection_speed 0.2))
  (return (Math|Random|RandomFloatinRange (- _cartridge_ejection_speed _returnvalue) (+ _cartridge_ejection_speed _returnvalue))))