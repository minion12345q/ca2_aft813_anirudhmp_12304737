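; BP_MP5 is the MP5 weapon Blueprint, firing automatically while fire is held.
; OnFireHeld checks readiness and ammo, then fires a raycast along the supplied forward vector, spends ammo, ejects a casing, animates the charger and starts the cooldown.
; A failed ammo check clears the ready flag without starting the cooldown.
; The fire pressed and left events are empty, and construction only calls the parent script.
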(event EventOnFireHeld
  (params (Forward%20Vector :type Vector :default "0, 0, 0"))
  (if (Variables|Default|GetIsReadyToFire)
    (bind _will_fire (CallFunction|CheckAmmoBeforeFiring))
    (if _will_fire
      (CallFunction|FireRayCast Forward%20Vector)
      (Variables|Default|SetIsReadyToFire false)
      (CallFunction|ReduceAmmoAfterFiring)
      (CallFunction|EjectCasing)
      (CallFunction|AnimateCharger)
      (CallFunction|StartWeaponCooldown)
      (else
        (Variables|Default|SetIsReadyToFire false)))))

(event EventOnFirePressed
  (params (Forward%20Vector :type Vector :default "0, 0, 0")))

(event EventOnFireLeft)

(fn ConstructionScript
  (|CallParentFunction))