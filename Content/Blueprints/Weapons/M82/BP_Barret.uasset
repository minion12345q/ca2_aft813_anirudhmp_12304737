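; BP_Barret is the Barrett M82 weapon Blueprint, a single-shot raycast gun.
; A fire press, gated by readiness and an ammo check, fires the ray, spends ammo, ejects a casing, animates the charger and starts a cooldown.
; A failed ammo check only clears readiness, noted as a reload in progress.
; Held and release inputs are empty, and health component damage and death events only print debug strings.
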(event EDDamageTaken(CBP_Health)
  (Development|PrintString "Hello"))

(event EDDeath(CBP_Health)
  (Development|PrintString "end game"))

(event EventBeginPlay
  (|CallParentFunction) ; This node is disabled and will not be called.\nDrag off pins to build functionality.
)

(event EventOnFireHeld
  (params (Forward%20Vector :type Vector :default "0, 0, 0")))

(event EventOnFireLeft)

(event EventOnFirePressed
  (params (Forward%20Vector :type Vector :default "0, 0, 0"))
  (if (Variables|Default|GetIsReadyToFire)
    (bind _will_fire (CallFunction|CheckAmmoBeforeFiring))
    (if _will_fire
      (CallFunction|FireRayCast Forward%20Vector) ; Fires a Raycast and does damage if possible
      (Variables|Default|SetIsReadyToFire false)
      (CallFunction|ReduceAmmoAfterFiring)
      (CallFunction|EjectCasing)
      (CallFunction|AnimateCharger)
      (CallFunction|StartWeaponCooldown)
      (else
        (Variables|Default|SetIsReadyToFire false) ; Reload Going On
      ))
    (else
      (Development|PrintString "Gun Is Not Ready to Fire Yet"))))

(fn ConstructionScript
  (|CallParentFunction))